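; Platformer checkpoint that updates the player's respawn point when the third-person character overlaps its box trigger.
; Each overlap writes the RespawnTransform component's world transform to the game mode's SpawnTransform.
; A DoOnce then lets a timeline rotate the flag pole on first activation only, followed by a 2D sound and a radial burst effect at the respawn point.
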(event `self.Box.OnComponentBeginOverlap`
  (params (OverlappedComponent :type "PrimitiveComponent Object Reference") (OtherActor :type "Actor Object Reference") (OtherComp :type "PrimitiveComponent Object Reference") (OtherBodyIndex :type Integer) (bFromSweep :type Boolean) (SweepResult :type "HitResult Structure (by ref)"))
  (cast `/Game/ThirdPerson/Blueprints/BP_ThirdPersonCharacter` OtherActor)
  (bind _asbp_third_person_game_mode (cast `/Game/ThirdPerson/Blueprints/BP_ThirdPersonGameMode` (`GameplayStatics.GetGameMode`)))
  (set `/Game/ThirdPerson/Blueprints/BP_ThirdPersonGameMode.Spawn Transform` (`SceneComponent.K2_GetComponentToWorld` (`self.Respawn Transform`)) _asbp_third_person_game_mode)
  (`/Engine/EditorBlueprintResources/StandardMacros.DoOnce` false
    (:`Completed`
      (bind (_direction _flag_alpha_over_time) (`Timeline|Flag Rotate` :!via `PlayFromStart`)
        (:`Update`
          (`SceneComponent.K2_SetRelativeRotation` (`self.Flag Pole`) (`KismetMathLibrary.RLerp` (`self.Flag Rotate Start`) (`self.Flag Rotate End`) _flag_alpha_over_time) false false))
        (:`Finished`
          ; Play SFX & VFX
          (`GameplayStatics.PlaySound2D` "/Engine/VREditor/Sounds/UI/Enter_Simulate.Enter_Simulate" 1.0 1.0 0.0 null null)
          (`NiagaraFunctionLibrary.SpawnSystemAtLocation` "/Niagara/DefaultAssets/Templates/Systems/RadialBurst.RadialBurst" (`SceneComponent.K2_GetComponentLocation` (`self.Respawn Transform`))))))))

(fn `UserConstructionScript`)