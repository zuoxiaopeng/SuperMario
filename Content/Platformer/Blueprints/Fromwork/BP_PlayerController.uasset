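; Player controller for a Mario-style platformer that owns the player's coins, points and lives and shows the HUD on BeginPlay.
; Reaching the coin cap rolls over into an extra life with a 1-up sound, and running out of lives opens the main menu level.
; The pause input toggles a pause widget, mouse cursor and game pause, using cursor visibility as the toggle state and sharing its resume path with the Continue event.
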(event `self.ReceiveBeginPlay`
  ; Add HUD to Viewport
  (bind _returnvalue (`|CreateWidget` "/Game/Platformer/UI/WBP_HUD.WBP_HUD_C"))
  (`UserWidget.AddToViewport` _returnvalue 0))

(event `Continue`
  ; Pause Manu
  (`Widget.RemoveFromParent` (`self.Pause Menu`) :!label _label)
  (set `self.bShowMouseCursor` false)
  (`GameplayStatics.PlaySound2D` "/Game/Platformer/Audio/Mario_Pause.Mario_Pause" 1.0 1.0 0.0 null null)
  (`GameplayStatics.SetGamePaused` false))

(event `EnhancedInput|/Game/ThirdPerson/Input/Actions/IA_Pause`
  (params (ActionValue :type Boolean) (ElapsedSeconds :type "Float (double-precision)") (TriggeredSeconds :type "Float (double-precision)") (InputAction :type "InputAction Object Reference" :default "/Game/ThirdPerson/Input/Actions/IA_Pause.IA_Pause"))
  ; Pause Manu
  (:`Started`
    (if (`self.bShowMouseCursor`)
      (goto _label)
      (else
        (bind _returnvalue (`|CreateWidget` "/Game/Platformer/UI/WBP_Pause.WBP_Pause_C"))
        (bind _output_get (set `self.Pause Menu` _returnvalue))
        (`UserWidget.AddToViewport` _output_get 0)
        (set `self.bShowMouseCursor` true)
        (`GameplayStatics.PlaySound2D` "/Game/Platformer/Audio/Mario_Pause.Mario_Pause" 1.0 1.0 0.0 null null)
        (`GameplayStatics.SetGamePaused` true)))))

(event `Add coins`
  (params (`Add Coins` :type Integer))
  (bind _returnvalue (+ `Add Coins` (`self.Coins`)))
  ; Add Coins
  (if (>= _returnvalue 100)
    (set `self.Coins` (`KismetMathLibrary.Clamp` (- _returnvalue 100) 0 100))
    (`self.Adjust Lives` 1)
    (`GameplayStatics.PlaySound2D` "/Game/Platformer/Audio/Mario_1up.Mario_1up" 1.0 1.0 0.0 null null)
    (else
      (set `self.Coins` (`KismetMathLibrary.Clamp` _returnvalue 0 100)))))

(event `Add Points`
  (params (`Points to Add` :type Integer))
  ; Add Points
  (set `self.Points` (+ `Points to Add` (`self.Points`))))

(event `Adjust Lives`
  (params (`Lives to Add or Subtract` :type Integer))
  ; Adjust Lives
  (bind _output_get (set `self.Lives` (`KismetMathLibrary.Clamp` (+ `Lives to Add or Subtract` (`self.Lives`)) 0 10)))
  (if (== _output_get 0)
    (`GameplayStatics.OpenLevel` "LV_MainMenu")))

(fn `UserConstructionScript`)