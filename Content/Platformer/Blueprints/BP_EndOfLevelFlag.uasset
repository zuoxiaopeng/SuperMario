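; End-of-level flagpole, styled on Mario, that ends the level when the player overlaps it.
; It disables input, calls level complete, then once snaps player and flag into place and suspends character movement.
; Chained MoveComponentTo calls slide both down, then fly the player to a celebration pose.
; If the level time's last digit equals FireworkShowSpecial, a self-calling DoN loop spawns that many random point-awarding fireworks.
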(event `self.ReceiveBeginPlay`
  ; Ref to Player Controller
  (bind _asbp_player_controller (cast `/Game/Platformer/Blueprints/Fromwork/BP_PlayerController` (`GameplayStatics.GetPlayerController` 0)))
  (set `self.My Controller` _asbp_player_controller))

(event `self.Triggle Volume.OnComponentBeginOverlap`
  (params (OverlappedComponent :type "PrimitiveComponent Object Reference") (OtherActor :type "Actor Object Reference") (OtherComp :type "PrimitiveComponent Object Reference") (OtherBodyIndex :type Integer) (bFromSweep :type Boolean) (SweepResult :type "HitResult Structure (by ref)"))
  (bind _flag_end_point (`self.Flag End Point`))
  (bind _my_charactor (`self.My Charactor`))
  (bind _player_explode_point (`self.Player Explode Point`))
  (bind _my_charactor_2 (`self.My Charactor`))
  (bind _fireworks_area (`self.Fireworks Area`))
  (bind _firework_points (`self.Firework Points`))
  (bind _firework_local (`self.Firework Local`))
  (bind _flag (`self.Flag`))
  (bind _player_end_point (`self.Player End Point`))
  (bind _returnvalue (`SceneComponent.K2_GetComponentRotation` (`self.Player End Point`)))
  (bind _charactermovement (`Character.CharacterMovement` (`self.My Charactor`)))
  (bind _mesh (`Character.Mesh` (`self.My Charactor`)))
  (bind _capsulecomponent (`Character.CapsuleComponent` (`self.My Charactor`)))
  (bind _x (.x (`SceneComponent.K2_GetComponentLocation` (`self.Flag`))))
  (bind _y (.y (`SceneComponent.K2_GetComponentLocation` (`self.Flag`))))
  (bind _z (.z (`SceneComponent.K2_GetComponentLocation` (`self.Flag`))))
  (bind _z_2 (.z (`SceneComponent.K2_GetComponentLocation` (`/Game/ThirdPerson/Blueprints/BP_ThirdPersonCharacter.Flag Attach Point` (`self.My Charactor`)))))
  ; Detect Player Overlap Flag Pole
  (bind _asbp_third_person_character (cast `/Game/ThirdPerson/Blueprints/BP_ThirdPersonCharacter` OtherActor))
  (bind _output_get (set `self.My Charactor` _asbp_third_person_character))
  (`self.DisableInput` _output_get (`GameplayStatics.GetPlayerController` 0))
  (`self.Level Complete !`)
  (`/Engine/EditorBlueprintResources/StandardMacros.DoOnce` false
    (:`Completed`
      ; Correction Flag Loc
      (if (< _z _z_2)
        (bind _output_get_2 (set `self.Flag Start Point` (`KismetMathLibrary.MakeVector` _x _y _z)))
        (`SceneComponent.K2_SetWorldLocation` _flag _output_get_2 false false)
        ; Correction Player Loc
        (`SceneComponent.K2_SetWorldLocationAndRotation` (`Character.CapsuleComponent` (`self.My Charactor`)) (`SceneComponent.K2_GetComponentLocation` (`self.Player Start Point`)) _returnvalue false false)
        (else
          (bind _output_get_3 (set `self.Flag Start Point` (`KismetMathLibrary.MakeVector` _x _y _z_2)))
          (`SceneComponent.K2_SetWorldLocation` _flag _output_get_3 false false)
          ; Set Charactor Position & Play Anim
          (`SceneComponent.K2_SetWorldRotation` _capsulecomponent _returnvalue false false)
          (`SceneComponent.K2_AddLocalOffset` _capsulecomponent (-45.0 0.0 -0.0) false false)))
      (set `CharacterMovementComponent.GravityScale` 0.0 _charactermovement)
      (`ActorComponent.Deactivate` _charactermovement)
      (`SkeletalMeshComponent.PlayAnimation` _mesh "/Game/LearningKit_Games/Assets/Characters/Character/Animations/epicCharacter_Interact_Start.EpicCharacter_Interact_Start" false)
      (`SkeletalMeshComponent.SetPosition` _mesh 0.83 true)
      ; Move Down Pole & Play SFX
      (`KismetSystemLibrary.Delay` 0.8)
      (`GameplayStatics.PlaySound2D` "/Game/Platformer/Audio/Mario_FlagPole.Mario_FlagPole" 1.0 1.0 0.0 null null)
      (`|ExecutionSequence`
        (:`then_0`
          (`KismetSystemLibrary.MoveComponentTo` (`Character.CapsuleComponent` (`self.My Charactor`)) (`SceneComponent.K2_GetComponentLocation` _player_end_point) (`SceneComponent.K2_GetComponentRotation` _player_end_point) false false 1.0)
          ; Fly to Sky & Play FX
          (`SkeletalMeshComponent.PlayAnimation` (`Character.Mesh` (`self.My Charactor`)) "/Game/LearningKit_Games/Assets/Characters/Character/Animations/epicCharacter_CrouchIdle.EpicCharacter_CrouchIdle" false)
          (`KismetSystemLibrary.Delay` 0.3)
          (`SkeletalMeshComponent.PlayAnimation` (`Character.Mesh` _my_charactor) "/Game/LearningKit_Games/Assets/Characters/Character/Animations/epicCharacter_FlySmooth.EpicCharacter_FlySmooth" false)
          (`KismetSystemLibrary.MoveComponentTo` (`Character.CapsuleComponent` _my_charactor) (`SceneComponent.K2_GetComponentLocation` _player_explode_point) (`SceneComponent.K2_GetComponentRotation` _player_explode_point) false false 0.5)
          (`SkeletalMeshComponent.PlayAnimation` (`Character.Mesh` _my_charactor_2) "/Game/LearningKit_Games/Assets/Characters/Character/Animations/epicCharacter_Celebrate.EpicCharacter_Celebrate" true)
          (`SceneComponent.K2_SetRelativeRotation` (`Character.CapsuleComponent` _my_charactor_2) (struct :`Yaw` 90.0) false false)
          (if (== (`self.Firework Show Special #`) (`KismetStringLibrary.Right` (`KismetStringLibrary.Conv_IntToString` (`/Game/Platformer/Blueprints/Fromwork/BP_PlayerController.Level Time` (`self.My Controller`))) 1))
            ; Play Firework
            (`KismetSystemLibrary.Delay` 0.5 :!label _label)
            (`/Engine/EditorBlueprintResources/StandardMacros.Do N` (`self.Firework Show Special #`)
              (:`Exit`
                (bind _output_get_4 (set `self.Firework Local` (`KismetMathLibrary.RandomPointInBoundingBox` (`SceneComponent.K2_GetComponentLocation` _fireworks_area) (`BoxComponent.BoxExtent` _fireworks_area))))
                (`GameplayStatics.SpawnEmitterAtLocation` "/Game/Realistic_Starter_VFX_Pack_Vol2/Particles/Sparks/P_Sparks_E.P_Sparks_E" _output_get_4)
                (`GameplayStatics.PlaySoundAtLocation` "/Game/Platformer/Audio/Mario_Thwomp.Mario_Thwomp" _firework_local (struct) 1.0 1.0 0.0 null null null null)
                (`|SpawnActorFromClass` "/Game/Platformer/Blueprints/BP_Points.BP_Points_C" (`KismetMathLibrary.MakeTransform` _firework_local) "Undefined" "MultiplyWithRoot" null _firework_points null)
                (`/Game/Platformer/Blueprints/Fromwork/BP_PlayerController.Add Points` (`self.My Controller`) _firework_points)
                (`self.More Firework`)))))
        (:`then_1`
          (`KismetSystemLibrary.MoveComponentTo` (`self.Flag`) (`SceneComponent.RelativeLocation` _flag_end_point) (`SceneComponent.RelativeRotation` _flag_end_point) false false 1.0))))))

(event `More Firework`
  (goto _label))

(fn `UserConstructionScript`)