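; Mario-style warp pipe that carries the third-person character to WarpToLocal.
; Collision overlap opens a gate so Up or Down input, chosen by IsDownPipe, triggers the warp when CanInteract is set.
; Input is disabled while timelines slide the player in, then out either rising or falling, with warp sounds.
; The construction script stacks instanced pipe segments downward based on PipeEndPoint's length.
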(event `EnhancedInput|/Game/ThirdPerson/Input/Actions/IA_PlayerUp`
  (params (ActionValue :type Boolean) (ElapsedSeconds :type "Float (double-precision)") (TriggeredSeconds :type "Float (double-precision)") (InputAction :type "InputAction Object Reference" :default "/Game/ThirdPerson/Input/Actions/IA_PlayerUp.IA_PlayerUp"))
  (:`Triggered`
    (if (and (`self.Can Interact ?`) (not (`self.is Down Pipe ?`)))
      (`/Engine/EditorBlueprintResources/StandardMacros.Gate` true :!label _label
        (:`Exit`
          (`self.DisableInput` (stale `self.Collision.OnComponentBeginOverlap` _output_get) (`GameplayStatics.GetPlayerController` 0))
          (if (`self.is Down Pipe ?`)
            (`|ExecutionSequence`
              (:`then_0`
                ; 0) Enter Down Pipe
                (bind (_direction _movement) (`Timeline|Into Down Pipe` :!via `PlayFromStart`)
                  (:`Update`
                    (`SceneComponent.K2_SetRelativeLocationAndRotation` :`self` (`Character.CapsuleComponent` (`self.My Player`)) :`NewLocation` (`KismetMathLibrary.MakeVector` (.x (`SceneComponent.K2_GetComponentLocation` (`self.Warp IN Point`))) (.y (`SceneComponent.K2_GetComponentLocation` (`self.Warp IN Point`))) (+ _movement (.z (`SceneComponent.K2_GetComponentLocation` (`self.Warp IN Point`)))))))
                  (:`Finished`
                    ; Wait a Bit Before Exiting Out of Pipe
                    (`KismetSystemLibrary.Delay` 0.4 :!label _label_2)
                    (`GameplayStatics.PlaySound2D` "/Game/Platformer/Audio/Mario_Warp.Mario_Warp" 1.0 1.0 0.0 null null)
                    (if (`self.Exits Falling Down Out of Pipe ?`)
                      ; Exits Falling Down Out of Pipe
                      (bind (_direction_2 _movement_2) (`Timeline|Timeline_0` :!via `PlayFromStart`)
                        (:`Update`
                          (`SceneComponent.K2_SetRelativeLocationAndRotation` :`self` (`Character.CapsuleComponent` (`self.My Player`)) :`NewLocation` (`KismetMathLibrary.MakeVector` (.x (`self.Warp to Local`)) (.y (`self.Warp to Local`)) (+ _movement_2 (.z (`self.Warp to Local`))))))
                        (:`Finished`
                          ; Enable Input again
                          (`self.EnableInput` (`self.My Player`) (`GameplayStatics.GetPlayerController` 0))))
                      (else
                        ; Exits Rising Up of Pipe
                        (bind (_direction_3 _movement_3) (`Timeline|Timeline_1` :!via `PlayFromStart`)
                          (:`Update`
                            (`SceneComponent.K2_SetRelativeLocationAndRotation` :`self` (`Character.CapsuleComponent` (`self.My Player`)) :`NewLocation` (`KismetMathLibrary.MakeVector` (.x (`self.Warp to Local`)) (.y (`self.Warp to Local`)) (+ _movement_3 (.z (`self.Warp to Local`))))))
                          (:`Finished`
                            ; Enable Input again
                            (`self.EnableInput` (`self.My Player`) (`GameplayStatics.GetPlayerController` 0)))))))))
              (:`then_1`
                ; 1) Play SFX
                (`KismetSystemLibrary.Delay` 0.2 :!label _label_3)
                (`GameplayStatics.PlaySound2D` "/Game/Platformer/Audio/Mario_Warp.Mario_Warp" 1.0 1.0 0.0 null null)))
            (else
              (`|ExecutionSequence`
                (:`then_0`
                  (goto _label_3))
                (:`then_1`
                  ; 0) Enter Down Pipe
                  (bind (_direction_4 _movement_4) (`Timeline|Timeline` :!via `PlayFromStart`)
                    (:`Update`
                      (`SceneComponent.K2_SetRelativeLocationAndRotation` :`self` (`Character.CapsuleComponent` (`self.My Player`)) :`NewLocation` (`KismetMathLibrary.MakeVector` (.x (`SceneComponent.K2_GetComponentLocation` (`self.Warp OUT Point`))) (.y (`SceneComponent.K2_GetComponentLocation` (`self.Warp OUT Point`))) (+ _movement_4 (.z (`SceneComponent.K2_GetComponentLocation` (`self.Warp OUT Point`)))))))
                    (:`Finished`
                      (goto _label_2))))))))))))

(event `EnhancedInput|/Game/ThirdPerson/Input/Actions/IA_PlayerDown`
  (params (ActionValue :type Boolean) (ElapsedSeconds :type "Float (double-precision)") (TriggeredSeconds :type "Float (double-precision)") (InputAction :type "InputAction Object Reference" :default "/Game/ThirdPerson/Input/Actions/IA_PlayerDown.IA_PlayerDown"))
  (:`Triggered`
    (if (and (`self.Can Interact ?`) (`self.is Down Pipe ?`))
      (goto _label))))

(event `self.Collision.OnComponentBeginOverlap`
  (params (OverlappedComponent :type "PrimitiveComponent Object Reference") (OtherActor :type "Actor Object Reference") (OtherComp :type "PrimitiveComponent Object Reference") (OtherBodyIndex :type Integer) (bFromSweep :type Boolean) (SweepResult :type "HitResult Structure (by ref)"))
  (bind _asbp_third_person_character (cast `/Game/ThirdPerson/Blueprints/BP_ThirdPersonCharacter` OtherActor))
  (bind _output_get (set `self.My Player` _asbp_third_person_character))
  (goto _label :!via `Open`))

(event `self.Collision.OnComponentEndOverlap`
  (params (OverlappedComponent :type "PrimitiveComponent Object Reference") (OtherActor :type "Actor Object Reference") (OtherComp :type "PrimitiveComponent Object Reference") (OtherBodyIndex :type Integer))
  (bind _asbp_third_person_character (cast `/Game/ThirdPerson/Blueprints/BP_ThirdPersonCharacter` OtherActor))
  (set `self.My Player` _asbp_third_person_character)
  (goto _label :!via `Close`))

(fn `UserConstructionScript`
  (for _index (range (+ (`KismetMathLibrary.FTrunc` (/ (`KismetMathLibrary.VSize` (`self.Pipe End Point`)) 100.0)) 1))
    (`InstancedStaticMeshComponent.AddInstance` (`self.Pipe Body`) (`KismetMathLibrary.MakeTransform` (`KismetMathLibrary.MakeVector` 0.0 0.0 (`KismetMathLibrary.Conv_IntToDouble` (* _index -100)))) false)))