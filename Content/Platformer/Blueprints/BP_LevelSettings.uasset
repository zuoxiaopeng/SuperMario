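; BP_LevelSettings runs a platformer level's music, countdown timer and completion flow.
; BeginPlay and respawns share one setup that resets the controller's time, starts music and timer, and binds game mode, character and flag events.
; The timer plays a low-time warning, raises music pitch, and kills the player at zero.
; Completion converts leftover time to points in a delay loop, saves stats to the GameInstance, and opens the next level.
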(event `Player Respawned_Event`
  ; 0) Playe Level Music
  (`AudioComponent.SetPitchMultiplier` (`self.Level Music Component`) 1.0)
  (`self.Player Respawned`))

(event `Player Respawned`
  (`|ExecutionSequence` :!label _label
    (:`then_0`
      ; 0) Playe Level Music
      (bind _asbp_third_person_game_mode (cast `/Game/ThirdPerson/Blueprints/BP_ThirdPersonGameMode` (`GameplayStatics.GetGameMode`)))
      (add `/Game/ThirdPerson/Blueprints/BP_ThirdPersonGameMode.Player Respawned` _asbp_third_person_game_mode (delegate `Player Respawned_Event`)))
    (:`then_1`
      ; 1) Ref to BP_PlayerController & Set Level Time variable
      (bind _asbp_player_controller (cast `/Game/Platformer/Blueprints/Fromwork/BP_PlayerController` (`GameplayStatics.GetPlayerController` 0)))
      (bind _output_get (set `self.Player Controller` _asbp_player_controller))
      (bind _output_get_2 (set `/Game/Platformer/Blueprints/Fromwork/BP_PlayerController.Level Time` (`self.Time Limit Max`) _output_get))
      (set `self.Time Limit Current` _output_get_2))
    (:`then_2`
      ; 2) Set Level Music
      (`AudioComponent.SetSound` (`self.Level Music Component`) (`self.Level Music`))
      (`KismetSystemLibrary.Delay` 0.75)
      (`AudioComponent.Play` (`self.Level Music Component`) 0.0))
    (:`then_3`
      ; 3) Run Timer & Play Appropriate Music Depending on the Situation
      (`KismetSystemLibrary.RetriggerableDelay` 1.0)
      (bind _returnvalue (`KismetSystemLibrary.K2_SetTimerDelegate` (delegate `Run Level Timer`) 1.0 true))
      (bind _output_get_3 (set `self.Level Timer` _returnvalue)))
    (:`then_4`
      ; 4) Stop Music & Timer if Player Has Died
      (bind _asbp_third_person_character (cast `/Game/ThirdPerson/Blueprints/BP_ThirdPersonCharacter` (`GameplayStatics.GetPlayerCharacter` 0)))
      (add `/Game/ThirdPerson/Blueprints/BP_ThirdPersonCharacter.Player Starts Death Sequence` _asbp_third_person_character (delegate `Player Starts Death Sequence_Event`)))
    (:`then_5`
      ; 4) Stop Mus & Timer & Add Points When Level Complete
      (add `/Game/Platformer/Blueprints/BP_EndOfLevelFlag.Level Complete !` (`self.End of Level Flag`) (delegate `Level Complete !_Event`)))))

(event `Run Level Timer`
  (bind _time_limit_current (`self.Time Limit Current`))
  (bind _level_music_component (`self.Level Music Component`))
  ; 3) Run Timer & Play Appropriate Music Depending on the Situation
  (if (== _time_limit_current 0)
    (`KismetSystemLibrary.K2_ClearAndInvalidateTimerHandle` (stale `Player Respawned` _output_get_3))
    (`AudioComponent.Stop` (`self.Level Music Component`))
    (`AudioComponent.Stop` (`self.Time Running Out Warning`))
    (bind _asbp_third_person_character (cast `/Game/ThirdPerson/Blueprints/BP_ThirdPersonCharacter` (`GameplayStatics.GetPlayerCharacter` 0)))
    (`/Game/ThirdPerson/Blueprints/BP_ThirdPersonCharacter.Player Dies` _asbp_third_person_character)
    (else
      (bind _result (`/Engine/EditorBlueprintResources/StandardMacros.DecrementInt` _time_limit_current)
        (:`  `
          (set `/Game/Platformer/Blueprints/Fromwork/BP_PlayerController.Level Time` _result (`self.Player Controller`))
          (if (== _time_limit_current (`self.Time Running Out Warning var`))
            (`AudioComponent.SetPaused` (`self.Level Music Component`) true)
            (`AudioComponent.Play` (`self.Time Running Out Warning`) 0.0)
            (`KismetSystemLibrary.Delay` 2.8)
            (`AudioComponent.SetPaused` _level_music_component false)
            (`AudioComponent.SetPitchMultiplier` _level_music_component 1.1)))))))

(event `self.ReceiveBeginPlay`
  (goto _label))

(event `Player Starts Death Sequence_Event`
  ; 4) Stop Music & Timer if Player Has Died
  (`AudioComponent.Stop` (`self.Time Running Out Warning`))
  (`AudioComponent.Stop` (`self.Level Music Component`))
  (`KismetSystemLibrary.K2_ClearAndInvalidateTimerHandle` (`self.Level Timer`)))

(event `Level Complete !_Event`
  (bind _player_controller (`self.Player Controller`))
  (bind _player_controller_2 (`self.Player Controller`))
  (bind _asbp_game_instance (cast `/Game/Platformer/Blueprints/Fromwork/BP_GameInstance` (`GameplayStatics.GetGameInstance`) :!pure true))
  (bind _level_time (`/Game/Platformer/Blueprints/Fromwork/BP_PlayerController.Level Time` _player_controller))
  ; 4) Stop Mus & Timer & Add Points When Level Complete
  (`AudioComponent.Stop` (`self.Time Running Out Warning`))
  (`AudioComponent.Stop` (`self.Level Music Component`))
  (`KismetSystemLibrary.K2_ClearAndInvalidateTimerHandle` (`self.Level Timer`))
  (`KismetSystemLibrary.Delay` 2.8)
  (`ActorComponent.Activate` (`self.Level Complete`) false)
  (`KismetSystemLibrary.Delay` 0.05 :!label _label_2)
  (if (> _level_time 0)
    (`/Engine/EditorBlueprintResources/StandardMacros.DecrementInt` _level_time
      (:`  `
        (`/Game/Platformer/Blueprints/Fromwork/BP_PlayerController.Add Points` _player_controller 50)
        (`GameplayStatics.PlaySound2D` "/Engine/VREditor/Sounds/UI/Camera_Shutter.Camera_Shutter" 1.0 1.0 0.0 null null)
        (goto _label_2)))
    (else
      (`KismetSystemLibrary.Delay` 2.0)
      ; Keep Player Stats & Change Level
      (set `/Game/Platformer/Blueprints/Fromwork/BP_GameInstance.Coins` (`/Game/Platformer/Blueprints/Fromwork/BP_PlayerController.Coins` _player_controller_2) _asbp_game_instance)
      (set `/Game/Platformer/Blueprints/Fromwork/BP_GameInstance.Points` (`/Game/Platformer/Blueprints/Fromwork/BP_PlayerController.Points` _player_controller_2) _asbp_game_instance)
      (set `/Game/Platformer/Blueprints/Fromwork/BP_GameInstance.Lives` (`/Game/Platformer/Blueprints/Fromwork/BP_PlayerController.Lives` _player_controller_2) _asbp_game_instance)
      (set `/Game/Platformer/Blueprints/Fromwork/BP_GameInstance.is Changing Level ?` true _asbp_game_instance)
      (`KismetSystemLibrary.Delay` 2.0)
      (`GameplayStatics.OpenLevel` (`self.Level to Go to`)))))

(fn `UserConstructionScript`)