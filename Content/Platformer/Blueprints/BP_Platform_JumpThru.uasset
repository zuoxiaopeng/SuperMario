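; One-way platform actor that lets the player jump up through it from below and drop down through it from on top.
; Overlapping the bottom trigger disables the Platform's collision, and leaving that trigger restores it.
; The top trigger tracks whether the player is standing above, allowing the IA_PlayerDown input to disable collision for a drop.
; Triggers react only to player 0's character.
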(event `self.Collision Bottom.OnComponentBeginOverlap`
  (params (OverlappedComponent :type "PrimitiveComponent Object Reference") (OtherActor :type "Actor Object Reference") (OtherComp :type "PrimitiveComponent Object Reference") (OtherBodyIndex :type Integer) (bFromSweep :type Boolean) (SweepResult :type "HitResult Structure (by ref)"))
  ; Jump up THROUGH Plantform
  (if (== OtherActor (`GameplayStatics.GetPlayerCharacter` 0))
    (`PrimitiveComponent.SetCollisionEnabled` (`self.Platform`) "NoCollision")))

(event `self.Collision Bottom.OnComponentEndOverlap`
  (params (OverlappedComponent :type "PrimitiveComponent Object Reference") (OtherActor :type "Actor Object Reference") (OtherComp :type "PrimitiveComponent Object Reference") (OtherBodyIndex :type Integer))
  ; Jump up THROUGH Plantform
  (if (== (`GameplayStatics.GetPlayerCharacter` 0) OtherActor)
    (`PrimitiveComponent.SetCollisionEnabled` (`self.Platform`) "QueryAndPhysics")))

(event `self.Collision Top.OnComponentBeginOverlap`
  (params (OverlappedComponent :type "PrimitiveComponent Object Reference") (OtherActor :type "Actor Object Reference") (OtherComp :type "PrimitiveComponent Object Reference") (OtherBodyIndex :type Integer) (bFromSweep :type Boolean) (SweepResult :type "HitResult Structure (by ref)"))
  ; Set Boolean for Detecting if Player is on TOP of Plantform
  (if (== OtherActor (`GameplayStatics.GetPlayerCharacter` 0))
    (set `self.is on Top of Plantform ?` true)))

(event `self.Collision Top.OnComponentEndOverlap`
  (params (OverlappedComponent :type "PrimitiveComponent Object Reference") (OtherActor :type "Actor Object Reference") (OtherComp :type "PrimitiveComponent Object Reference") (OtherBodyIndex :type Integer))
  ; Set Boolean for Detecting if Player is on TOP of Plantform
  (if (== (`GameplayStatics.GetPlayerCharacter` 0) OtherActor)
    (set `self.is on Top of Plantform ?` false)))

(event `EnhancedInput|/Game/ThirdPerson/Input/Actions/IA_PlayerDown`
  (params (ActionValue :type Boolean) (ElapsedSeconds :type "Float (double-precision)") (TriggeredSeconds :type "Float (double-precision)") (InputAction :type "InputAction Object Reference" :default "/Game/ThirdPerson/Input/Actions/IA_PlayerDown.IA_PlayerDown"))
  ; Allow Player to Drop Down Through The Plantform
  (:`Triggered`
    (if (`self.is on Top of Plantform ?`)
      (`PrimitiveComponent.SetCollisionEnabled` (`self.Platform`) "NoCollision"))))

(fn `UserConstructionScript`)