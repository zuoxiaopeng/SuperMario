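; Base platformer block that reacts to the character hitting it from below and can swap between a solid block and a coin.
; An upward hit normal on the cube stops the jump, slams the character downward and calls HitBlockMessage, debounced by a DoOnce with a short delay.
; PBlock On and Off toggle cube visibility and collision against the coin child actor.
; Player overlap with the coin collider destroys the whole actor.
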(event `self.ReceiveBeginPlay`
  ; Reference to PlayerController
  (bind _asbp_player_controller (cast `/Game/Platformer/Blueprints/Fromwork/BP_PlayerController` (`GameplayStatics.GetPlayerController` 0)))
  (set `self.Player Controller` _asbp_player_controller))

(event `self.Cube.OnComponentHit`
  (params (HitComponent :type "PrimitiveComponent Object Reference") (OtherActor :type "Actor Object Reference") (OtherComp :type "PrimitiveComponent Object Reference") (NormalImpulse :type "Vector Structure") (Hit :type "HitResult Structure (by ref)"))
  ; Block Hit From Bottom
  (bind _asbp_third_person_character (cast `/Game/ThirdPerson/Blueprints/BP_ThirdPersonCharacter` OtherActor))
  (if (== (.z (`.ImpactNormal` (`GameplayStatics.BreakHitResult` Hit))) 1.0)
    (`Character.StopJumping` _asbp_third_person_character)
    (set `MovementComponent.Velocity` (0.0 0.0 -1000.0) (`Character.CharacterMovement` _asbp_third_person_character))
    (`/Engine/EditorBlueprintResources/StandardMacros.DoOnce` false :!label _label
      (:`Completed`
        (message `/Game/Platformer/Blueprints/BPI_Platform.Hit Block` self)
        (`KismetSystemLibrary.Delay` 0.2)
        (goto _label :!via `Reset`)))))

(event `self.Coin Collider.OnComponentBeginOverlap`
  (params (OverlappedComponent :type "PrimitiveComponent Object Reference") (OtherActor :type "Actor Object Reference") (OtherComp :type "PrimitiveComponent Object Reference") (OtherBodyIndex :type Integer) (bFromSweep :type Boolean) (SweepResult :type "HitResult Structure (by ref)"))
  (if (== OtherActor (`GameplayStatics.GetPlayerCharacter` 0))
    (`self.K2_DestroyActor`)))

(fn `PBlock Off`
  (bind _cube (`self.Cube`))
  ; Show off Block
  (`SceneComponent.SetVisibility` _cube true false)
  (`PrimitiveComponent.SetCollisionEnabled` _cube "QueryAndPhysics")
  (`SceneComponent.SetVisibility` (`self.ChildActor`) false false))

(fn `PBlock On`
  (bind _cube (`self.Cube`))
  ; Show off Coin
  (`SceneComponent.SetVisibility` _cube false false)
  (`PrimitiveComponent.SetCollisionEnabled` _cube "NoCollision")
  (`SceneComponent.SetVisibility` (`self.ChildActor`) true false))

(fn `UserConstructionScript`)