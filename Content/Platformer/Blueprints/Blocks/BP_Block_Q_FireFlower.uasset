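; Question block for a Mario-style platformer that reveals a Fire Flower power-up when hit.
; The first hit plays effects, swaps the cube material and runs timelines that bump the block and move the flower, then adds a glow emitter; later hits only play a bump sound.
; Overlapping the flower grants the character flower power, spawns a points actor, adds score and removes the flower and glow.
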(event `self.Hit Block`
  (if (`self.Finished Interacting ?`)
    (`GameplayStatics.PlaySound2D` "/Game/Platformer/Audio/Mario_BrickBump.Mario_BrickBump" 1.0 1.0 0.0 null null)
    (else
      (`|ExecutionSequence`
        (:`then_0`
          ; 0) Play FX
          (`/Game/Platformer/Blueprints/BP_Function_Library. Play Block Interact FX` (`self.Interact SFX`) null (`self.Interact VFX(Particle)`) (+ (`self.K2_GetActorLocation`) (0.0 0.0 50.0)))
          (`PrimitiveComponent.SetMaterial` (`self.Cube`) 0 (`self.Interact Material`)))
        (:`then_1`
          ; 1) Block Anim
          (bind (_direction _movement) (`Timeline|Block Anim` :!via `PlayFromStart`)
            (:`Update`
              (`SceneComponent.K2_SetRelativeLocation` (`self.Cube`) (`KismetMathLibrary.MakeVector` 0.0 0.0 _movement) false false))
            (:`Finished`
              (bind _returnvalue (`GameplayStatics.SpawnEmitterAtLocation` "/Game/Realistic_Starter_VFX_Pack_Vol2/Particles/Environment/P_Fireflies.P_Fireflies" (- (`SceneComponent.K2_GetComponentLocation` (`self.Box_Flower`)) (0.0 0.0 100.0))))
              (set `self.Power Up Glow` _returnvalue))))
        (:`then_2`
          ; 2) Flower Anim
          (bind (_direction_2 _flower_anim) (`Timeline|Flower Anim` :!via `PlayFromStart`)
            (:`Update`
              (bind _box_flower (`self.Box_Flower`)
                (:`then`
                  (`SceneComponent.K2_SetRelativeLocation` _box_flower (`KismetMathLibrary.MakeVector` 0.0 0.0 _flower_anim) false false))
                (:`else`)))))
        (:`then_3`
          (set `self.Finished Interacting ?` true))))))

(event `self.Box_Flower.OnComponentBeginOverlap`
  (params (OverlappedComponent :type "PrimitiveComponent Object Reference") (OtherActor :type "Actor Object Reference") (OtherComp :type "PrimitiveComponent Object Reference") (OtherBodyIndex :type Integer) (bFromSweep :type Boolean) (SweepResult :type "HitResult Structure (by ref)"))
  (bind _asbp_third_person_character (cast `/Game/ThirdPerson/Blueprints/BP_ThirdPersonCharacter` OtherActor))
  (`/Game/ThirdPerson/Blueprints/BP_ThirdPersonCharacter.Got Flower Power` _asbp_third_person_character)
  (`|ExecutionSequence`
    (:`then_0`
      ; 0) Add Points
      (`|SpawnActorFromClass` "/Game/Platformer/Blueprints/BP_Points.BP_Points_C" (`SceneComponent.K2_GetComponentToWorld` (`self.Arrow`)) "Undefined" "MultiplyWithRoot" null (`self.Points`) null)
      (`/Game/Platformer/Blueprints/Fromwork/BP_PlayerController.Add Points` (`self.Player Controller`) (`self.Points`)))
    (:`then_1`
      ; 1) Destory Flower Component
      (`ActorComponent.K2_DestroyComponent` (`self.Power Up Glow`)))
    (:`then_2`
      (`ActorComponent.K2_DestroyComponent` (`self.Mesh_Flower`))
      (`ActorComponent.K2_DestroyComponent` (`self.Box_Flower`)))))

(fn `UserConstructionScript`
  (`parent.UserConstructionScript`))