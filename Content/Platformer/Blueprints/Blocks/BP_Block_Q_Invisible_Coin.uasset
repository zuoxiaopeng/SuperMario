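; Invisible coin question block for a Mario-style platformer that stays hidden and ignores a custom trace channel (fireballs) until hit.
; A Box trigger disables the cube's collision while the player overlaps it.
; The first hit plays FX, awards points and coins, bounces the cube via timeline, reveals it with full blocking and removes the trigger.
; Later hits only play a bump sound.
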(event `self.ReceiveBeginPlay`
  (`parent.ReceiveBeginPlay`)
  ; not PBlock
  (`|ExecutionSequence`
    (:`then_0`
      ; Invisible & Ignore Fireball
      (`SceneComponent.SetVisibility` (`self.Cube`) false false)
      (`PrimitiveComponent.SetCollisionResponseToChannel` (`self.Cube`) "ECC_GameTraceChannel1" "ECR_Ignore"))
    (:`then_1`
      (`ActorComponent.K2_DestroyComponent` (`self.ChildActor`))
      (`ActorComponent.K2_DestroyComponent` (`self.Coin Collider`)))))

(event `self.Hit Block`
  (if (`self.Finished Interacting ?`)
    (`GameplayStatics.PlaySound2D` "/Game/Platformer/Audio/Mario_BrickBump.Mario_BrickBump" 1.0 1.0 0.0 null null)
    (else
      (`|ExecutionSequence`
        (:`then_0`
          ; 0) Play FX
          (`/Game/Platformer/Blueprints/BP_Function_Library. Play Block Interact FX` (`self.Interact SFX`) null (`self.Interact VFX(Particle)`) (+ (`self.K2_GetActorLocation`) (0.0 0.0 50.0)))
          (`PrimitiveComponent.SetMaterial` (`self.Cube`) 0 (`self.Interact Material`)))
        (:`then_1`
          ; 1) Add Points
          (`|SpawnActorFromClass` "/Game/Platformer/Blueprints/BP_Points.BP_Points_C" (`self.GetTransform`) "Undefined" "MultiplyWithRoot" null (`self.Points`) null)
          (`/Game/Platformer/Blueprints/Fromwork/BP_PlayerController.Add Points` (`self.Player Controller`) (`self.Points`)))
        (:`then_2`
          ; 2) Add Coins
          (`|SpawnActorFromClass` "/Game/Platformer/Blueprints/Blocks/BP_Block_Coin.BP_Block_Coin_C" (`self.GetTransform`) "Undefined" "MultiplyWithRoot" null null)
          (`/Game/Platformer/Blueprints/Fromwork/BP_PlayerController.Add coins` (`self.Player Controller`) (`self.Coins to Add`)))
        (:`then_3`
          ; 3) Block Anim
          (bind (_direction _movement) (`Timeline|Block Anim` :!via `PlayFromStart`)
            (:`Update`
              (`SceneComponent.K2_SetRelativeLocation` (`self.Cube`) (`KismetMathLibrary.MakeVector` 0.0 0.0 _movement) false false))))
        (:`then_4`
          ; 4) turn Visibility ON
          (`SceneComponent.SetVisibility` (`self.Cube`) true false)
          (`ActorComponent.K2_DestroyComponent` (`self.Box`))
          (`PrimitiveComponent.SetCollisionResponseToChannel` (`self.Cube`) "ECC_GameTraceChannel1" "ECR_Block"))
        (:`then_5`
          (set `self.Finished Interacting ?` true))))))

(event `self.Box.OnComponentBeginOverlap`
  (params (OverlappedComponent :type "PrimitiveComponent Object Reference") (OtherActor :type "Actor Object Reference") (OtherComp :type "PrimitiveComponent Object Reference") (OtherBodyIndex :type Integer) (bFromSweep :type Boolean) (SweepResult :type "HitResult Structure (by ref)"))
  ; Toggle Block Collision
  (if (== OtherActor (`GameplayStatics.GetPlayerCharacter` 0))
    (`PrimitiveComponent.SetCollisionEnabled` (`self.Cube`) "NoCollision")))

(event `self.Box.OnComponentEndOverlap`
  (params (OverlappedComponent :type "PrimitiveComponent Object Reference") (OtherActor :type "Actor Object Reference") (OtherComp :type "PrimitiveComponent Object Reference") (OtherBodyIndex :type Integer))
  ; Toggle Block Collision
  (if (== (`GameplayStatics.GetPlayerCharacter` 0) OtherActor)
    (`PrimitiveComponent.SetCollisionEnabled` (`self.Cube`) "QueryAndPhysics")))

(fn `UserConstructionScript`
  (`parent.UserConstructionScript`))