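; BP_Block_Coin is a short-lived coin effect for platformer blocks that animates a coin and then removes itself.
; On BeginPlay, the CoinAni timeline plays from the start, driving the Coin component's relative height and spin through its Movement and Rotation tracks.
; When the timeline finishes, it spawns a particle emitter at the coin's world location and destroys the actor.
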(event `self.ReceiveBeginPlay`
  ; Coin Anim
  (`TimelineComponent.SetPlayRate` (`self.Coin Ani`) 1.0)
  (bind (_direction _movement _rotation) (`Timeline|Coin Ani` :!via `PlayFromStart`)
    (:`Update`
      (`SceneComponent.K2_SetRelativeLocationAndRotation` (`self.Coin`) (`KismetMathLibrary.MakeVector` 0.0 0.0 _movement) (`KismetMathLibrary.MakeRotator` -70.0 -90.0 _rotation) false false))
    (:`Finished`
      (`GameplayStatics.SpawnEmitterAtLocation` null (`SceneComponent.K2_GetComponentLocation` (`self.Coin`)))
      (`self.K2_DestroyActor`))))

(fn `UserConstructionScript`)