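; BP_Block_Fake_Breakable is a platformer block that pays out points and a coin when hit, then becomes inert.
; On the first HitBlock it plays interact effects, swaps the cube's material, spawns points and coin actors, and credits both to the PlayerController.
; A BlockAnim timeline bumps the cube along Z.
; A FinishedInteracting flag makes later hits play only a brick bump sound.
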(event `self.Hit Block`
  (if (`self.Finished Interacting ?`)
    (`GameplayStatics.PlaySound2D` "/Game/Platformer/Audio/Mario_BrickBump.Mario_BrickBump" 1.0 1.0 0.0 null null)
    (else
      (`|ExecutionSequence`
        (:`then_0`
          ; 0) Play FX
          (`/Game/Platformer/Blueprints/BP_Function_Library. Play Block Interact FX` (`self.Interact SFX`) null (`self.Interact VFX(Particle)`) (+ (`self.K2_GetActorLocation`) (0.0 0.0 50.0)))
          (`PrimitiveComponent.SetMaterial` (`self.Cube`) 0 (`self.Interact Material`)))
        (:`then_1`
          ; 1) Add Points
          (`|SpawnActorFromClass` "/Game/Platformer/Blueprints/BP_Points.BP_Points_C" (`self.GetTransform`) "Undefined" "MultiplyWithRoot" null (`self.Points`) null)
          (`/Game/Platformer/Blueprints/Fromwork/BP_PlayerController.Add Points` (`self.Player Controller`) (`self.Points`)))
        (:`then_2`
          ; 2) Add Coins
          (`|SpawnActorFromClass` "/Game/Platformer/Blueprints/Blocks/BP_Block_Coin.BP_Block_Coin_C" (`self.GetTransform`) "Undefined" "MultiplyWithRoot" null null)
          (`/Game/Platformer/Blueprints/Fromwork/BP_PlayerController.Add coins` (`self.Player Controller`) (`self.Coins to Add`)))
        (:`then_3`
          ; 3) Block Anim
          (bind (_direction _movement) (`Timeline|Block Anim` :!via `PlayFromStart`)
            (:`Update`
              (`SceneComponent.K2_SetRelativeLocation` (`self.Cube`) (`KismetMathLibrary.MakeVector` 0.0 0.0 _movement) false false))))
        (:`then_4`
          (set `self.Finished Interacting ?` true))))))

(fn `UserConstructionScript`
  (`parent.UserConstructionScript`))