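; P-switch block for the platformer that, when stomped by the player, temporarily switches on tagged blocks.
; A downward-normal box hit bounces the character, plays effects, swaps to smashed meshes and pauses level music for its own track.
; It calls PBlockOn on tagged BP_Block_Base actors and starts a timer.
; Timeout, player death or level completion share one path that calls PBlockOff and restores the music.
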(event `self.Box.OnComponentHit`
  (params (HitComponent :type "PrimitiveComponent Object Reference") (OtherActor :type "Actor Object Reference") (OtherComp :type "PrimitiveComponent Object Reference") (NormalImpulse :type "Vector Structure") (Hit :type "HitResult Structure (by ref)"))
  (bind _asbp_third_person_character (cast `/Game/ThirdPerson/Blueprints/BP_ThirdPersonCharacter` OtherActor))
  (if (== (`.Normal` (`GameplayStatics.BreakHitResult` Hit)) (0.0 0.0 -1.0) :`ErrorTolerance` 0.1)
    (`Character.LaunchCharacter` _asbp_third_person_character (0.0 0.0 400.0) false false)
    (`|ExecutionSequence`
      (:`then_0`
        ; 0) PBlock FX
        (`GameplayStatics.PlaySound2D` "/Game/Platformer/Audio/Mario_Thwomp.Mario_Thwomp" 1.0 1.0 0.0 null null)
        (`GameplayStatics.SpawnEmitterAtLocation` "/Game/Realistic_Starter_VFX_Pack_Vol2/Particles/Hit/P_Ceramic.P_Ceramic" (`SceneComponent.K2_GetComponentLocation` (`self.Block_P_Base_Smashed`)))
        (`AudioComponent.Play` (`self.Music`) 0.0)
        (`AudioComponent.SetPaused` (`/Game/Platformer/Blueprints/BP_LevelSettings.Level Music Component` (`self.Level Settings`)) true))
      (:`then_1`
        ; 1) Camera Shake & Force Feedback
        (`GameplayStatics.PlayWorldCameraShake` "/Game/Platformer/Blueprints/Blocks/PBlock/BP_CameraShake.BP_CameraShake_C" (`self.K2_GetActorLocation` (`GameplayStatics.GetPlayerCharacter` 0)) 1000.0 2000.0)
        (`PlayerController.K2_ClientPlayForceFeedback` (`GameplayStatics.GetPlayerController` 0) "/Game/Platformer/Blueprints/Blocks/PBlock/ForceFeedBack.ForceFeedBack" "None" false false false))
      (:`then_2`
        ; 2) Show Meshes & Destroy Component
        (`SceneComponent.SetVisibility` (`self.Block_P_Base_Smashed`) true false)
        (`SceneComponent.SetVisibility` (`self.Block_P_Top_Smashed`) true false)
        (`ActorComponent.K2_DestroyComponent` (`self.Block_P`))
        (`ActorComponent.K2_DestroyComponent` (`self.Box`)))
      (:`then_3`
        ; 3) Find all Actor with PBlock Tag & Turn ON Function Found in the Parent Block
        (bind _outactors (`GameplayStatics.GetAllActorsWithTag` (`self.Tag`)))
        (bind _output_get (set `self.Blocks` _outactors))
        (for _array_element _output_get
          (bind _asbp_block_base (cast `/Game/Platformer/Blueprints/Blocks/BP_Block_Base` _array_element))
          (`/Game/Platformer/Blueprints/Blocks/BP_Block_Base.PBlock On` _asbp_block_base)))
      (:`then_4`
        ; 4) PBlock Timer
        (`KismetSystemLibrary.K2_SetTimerDelegate` (delegate `PBlock Time Over`) (`self.PBlock Time Duration`)))
      (:`then_5`
        (add `/Game/ThirdPerson/Blueprints/BP_ThirdPersonCharacter.Player Starts Death Sequence` _asbp_third_person_character (delegate `Player Starts Death Sequence_Event`)))
      (:`then_6`
        (add `/Game/Platformer/Blueprints/BP_EndOfLevelFlag.Level Complete !` (`self.End of Level Flag`) (delegate `Level Complete !_Event`))))))

(event `PBlock Time Over`
  ; 4) PBlock Timer
  (for _array_element (`self.Blocks`) :!label _label
    (bind _asbp_block_base (cast `/Game/Platformer/Blueprints/Blocks/BP_Block_Base` _array_element))
    (`/Engine/EditorBlueprintResources/StandardMacros.IsValid` _asbp_block_base
      (:`Is Valid`
        (`/Game/Platformer/Blueprints/Blocks/BP_Block_Base.PBlock Off` _asbp_block_base))
      (:`Is Not Valid`
        _))
    (`AudioComponent.Stop` (`self.Music`))
    (`AudioComponent.SetPaused` (`/Game/Platformer/Blueprints/BP_LevelSettings.Level Music Component` (`self.Level Settings`)) false)))

(event `Player Starts Death Sequence_Event`
  (goto _label))

(event `Level Complete !_Event`
  (goto _label))

(fn `UserConstructionScript`)