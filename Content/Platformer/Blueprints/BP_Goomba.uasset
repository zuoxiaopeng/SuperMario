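; BP_Goomba is a Mario-style flipbook enemy that damages the player on overlap and dies to stomps or fireballs.
; A gate opened by PlayerDetectRange runs its movement only while the player is near, either seeking the player or walking along X and flipping on wall hits.
; A top-down hit on StompBox squishes it before delayed destruction, while fireballs destroy it immediately; both award points.
; Construction derives flipbook play rate from walk speed.
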(event `self.ReceiveBeginPlay`
  ; Ref to Player Controller
  (bind _asbp_player_controller (cast `/Game/Platformer/Blueprints/Fromwork/BP_PlayerController` (`GameplayStatics.GetPlayerController` 0)))
  (set `self.Player Controller` _asbp_player_controller))

(event `self.Collider.OnComponentBeginOverlap`
  (params (OverlappedComponent :type "PrimitiveComponent Object Reference") (OtherActor :type "Actor Object Reference") (OtherComp :type "PrimitiveComponent Object Reference") (OtherBodyIndex :type Integer) (bFromSweep :type Boolean) (SweepResult :type "HitResult Structure (by ref)"))
  ; Gooba Dmage Player
  (bind _asbp_third_person_character (cast `/Game/ThirdPerson/Blueprints/BP_ThirdPersonCharacter` OtherActor))
  (`/Game/ThirdPerson/Blueprints/BP_ThirdPersonCharacter.Adjust Hit Points` _asbp_third_person_character (`self.Health to Subtruct`)))

(event `self.StompBox.OnComponentHit`
  (params (HitComponent :type "PrimitiveComponent Object Reference") (OtherActor :type "Actor Object Reference") (OtherComp :type "PrimitiveComponent Object Reference") (NormalImpulse :type "Vector Structure") (Hit :type "HitResult Structure (by ref)"))
  (bind _paperflipbook (`self.PaperFlipbook`))
  (if (and (== OtherActor (`GameplayStatics.GetPlayerCharacter` 0)) (== (`.Normal` (`GameplayStatics.BreakHitResult` Hit)) (0.0 0.0 -1.0)))
    (`|ExecutionSequence`
      (:`then_0`
        ; 0) Enem Squish FX
        (`GameplayStatics.PlaySound2D` "/Game/Platformer/Audio/Mario_Squish.Mario_Squish" 1.0 1.0 0.0 null null)
        (`PrimitiveComponent.SetCollisionEnabled` (`self.Collider`) "NoCollision")
        (`ActorComponent.K2_DestroyComponent` (`self.StompBox`))
        (`SceneComponent.SetWorldScale3D` _paperflipbook (0.25 0.25 0.1))
        (`SceneComponent.K2_AddWorldOffset` _paperflipbook (0.0 0.0 -35.0) false false)
        (`CharacterMovementComponent.DisableMovement` (`self.CharacterMovement`)))
      (:`then_1`
        ; 1) Add Points
        (`|SpawnActorFromClass` "/Game/Platformer/Blueprints/BP_Points.BP_Points_C" (`self.GetTransform`) "Undefined" "MultiplyWithRoot" null (`self.Points`) null)
        (`/Game/Platformer/Blueprints/Fromwork/BP_PlayerController.Add Points` (`self.Player Controller`) (`self.Points`)))
      (:`then_2`
        ; 2) Play FX & Destory Goomba
        (`KismetSystemLibrary.Delay` 0.5)
        (`/Game/Platformer/Blueprints/BP_Function_Library. Play Block Interact FX` "/Game/Platformer/Audio/Mario_Kick.Mario_Kick" null "/Game/Realistic_Starter_VFX_Pack_Vol2/Particles/Destruction/P_Destruction_Wood.P_Destruction_Wood" (`SceneComponent.K2_GetComponentLocation` (`self.Collider`)))
        (`self.K2_DestroyActor`)))))

(event `self.Collider.OnComponentHit`
  (params (HitComponent :type "PrimitiveComponent Object Reference") (OtherActor :type "Actor Object Reference") (OtherComp :type "PrimitiveComponent Object Reference") (NormalImpulse :type "Vector Structure") (Hit :type "HitResult Structure (by ref)"))
  (bind _asbp_fireball (cast `/Game/Platformer/Blueprints/BP_Fireball` OtherActor))
  (`self.K2_DestroyActor` _asbp_fireball)
  (`|ExecutionSequence`
    (:`then_0`
      ; 0) Add Points
      (`|SpawnActorFromClass` "/Game/Platformer/Blueprints/BP_Points.BP_Points_C" (`self.GetTransform`) "Undefined" "MultiplyWithRoot" null (`self.Points`) null)
      (`/Game/Platformer/Blueprints/Fromwork/BP_PlayerController.Add Points` (`self.Player Controller`) (`self.Points`)))
    (:`then_1`
      ; 1) Play FX & Destory Goomba
      (`/Game/Platformer/Blueprints/BP_Function_Library. Play Block Interact FX` "/Game/Platformer/Audio/Mario_Kick.Mario_Kick" null "/Game/Realistic_Starter_VFX_Pack_Vol2/Particles/Destruction/P_Destruction_Wood.P_Destruction_Wood" (`SceneComponent.K2_GetComponentLocation` (`self.Collider`)))
      (`self.K2_DestroyActor`))))

(event `self.ReceiveTick`
  (params (DeltaSeconds :type "Float (single-precision)"))
  ; Move Gooba Give a Direction Only IF Player is in Range
  (`/Engine/EditorBlueprintResources/StandardMacros.Gate` true :!label _label
    (:`Exit`
      (if (`self.is Seeker Enemy ?`)
        (`AIBlueprintHelperLibrary.SimpleMoveToActor` (`self.GetController`) (`GameplayStatics.GetPlayerCharacter` 0))
        (else
          (`self.AddMovementInput` (select `bool` (`self.Move Left ?`) :`false` (1.0 0.0 0.0) :`true` (-1.0 0.0 0.0) :!type "Vector Structure"))
          (`PaperFlipbookComponent.SetPlayRate` (`self.PaperFlipbook`) (`self.Flipbook Play Rate Multiply`)))))))

(event `self.Player Detect Range.OnComponentBeginOverlap`
  (params (OverlappedComponent :type "PrimitiveComponent Object Reference") (OtherActor :type "Actor Object Reference") (OtherComp :type "PrimitiveComponent Object Reference") (OtherBodyIndex :type Integer) (bFromSweep :type Boolean) (SweepResult :type "HitResult Structure (by ref)"))
  ; Move Gooba Give a Direction Only IF Player is in Range
  (cast `/Game/ThirdPerson/Blueprints/BP_ThirdPersonCharacter` OtherActor)
  (goto _label :!via `Open`))

(event `self.Player Detect Range.OnComponentEndOverlap`
  (params (OverlappedComponent :type "PrimitiveComponent Object Reference") (OtherActor :type "Actor Object Reference") (OtherComp :type "PrimitiveComponent Object Reference") (OtherBodyIndex :type Integer))
  ; Move Gooba Give a Direction Only IF Player is in Range
  (cast `/Game/ThirdPerson/Blueprints/BP_ThirdPersonCharacter` OtherActor)
  (goto _label :!via `Close`))

(event `self.CapsuleComponent.OnComponentHit`
  (params (HitComponent :type "PrimitiveComponent Object Reference") (OtherActor :type "Actor Object Reference") (OtherComp :type "PrimitiveComponent Object Reference") (NormalImpulse :type "Vector Structure") (Hit :type "HitResult Structure (by ref)"))
  ; Goomba Turn Back
  (`/Engine/EditorBlueprintResources/StandardMacros.DoOnce` false :!label _label_2
    (:`Completed`
      (if (== (`KismetMathLibrary.Vector_GetAbs` (`.Normal` (`GameplayStatics.BreakHitResult` Hit))) (1.0 0.0 0.0) :`ErrorTolerance` 0.1)
        (`/Engine/EditorBlueprintResources/StandardMacros.FlipFlop`
          (:`A`
            (set `self.Move Left ?` true))
          (:`B`
            (set `self.Move Left ?` false)))
        (`KismetSystemLibrary.Delay` 0.2)
        (goto _label_2 :!via `Reset`)))))

(fn `UserConstructionScript`
  (bind _output_get (set `CharacterMovementComponent.MaxWalkSpeed` (`self.Speed`) (`self.CharacterMovement`)))
  (set `self.Flipbook Play Rate Multiply` (`KismetMathLibrary.FClamp` (/ _output_get 100.0) 0.1 3.0)))