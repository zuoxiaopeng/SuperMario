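; BP_Cloud is a scenery actor that fills a box volume with randomly scattered clouds.
; Its Construction Script sizes the SpawnArea box from the exposed extents, then adds CloudNum instances to the Cloud instanced mesh component at random points inside it.
; Each instance gets a fixed rotation and a random uniform scale between ScaleMin and ScaleMax.
; The event graph is empty, so the clouds have no runtime logic.
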(fn `UserConstructionScript`
  (bind _spawn_area (`self.Spawn Area`))
  (`BoxComponent.SetBoxExtent` (`self.Spawn Area`) (`KismetMathLibrary.MakeVector` (`self.Spawn Area X`) (`self.Spawn Area Y`) (`self.Spawn Area Z`)) true)
  (for _ (range 1 (+ (`self.Cloud Num`) 1))
    (`InstancedStaticMeshComponent.AddInstance` (`self.Cloud`) (`KismetMathLibrary.MakeTransform` (`KismetMathLibrary.RandomPointInBoundingBox` (`SceneComponent.RelativeLocation` _spawn_area) (`BoxComponent.BoxExtent` _spawn_area)) (struct :`Roll` 90.0) (`KismetMathLibrary.Conv_DoubleToVector` (`KismetMathLibrary.RandomFloatInRange` (`self.Scale Min`) (`self.Scale Max`)))) false)))