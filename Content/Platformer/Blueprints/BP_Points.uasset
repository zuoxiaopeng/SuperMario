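; BP_Points is a short-lived floating score popup actor that shows a points value through a widget component.
; On BeginPlay it gets its WBP_Points widget, plays the points animation and sets the text to PointsToAdd.
; It waits for the animation's end time, then destroys itself.
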(event `self.ReceiveBeginPlay`
  ; Play Points Animation
  (bind _aswbp_points (cast `/Game/Platformer/UI/WBP_Points` (`WidgetComponent.GetWidget` (`self.Text_Widget`))))
  (bind _points_animation (`/Game/Platformer/UI/WBP_Points.Points_Animation` _aswbp_points))
  (`UserWidget.PlayAnimation` _aswbp_points _points_animation 0.0 1 "Forward" 1.0 false)
  (`TextBlock.SetText` (`/Game/Platformer/UI/WBP_Points.Points_text` _aswbp_points) (`KismetTextLibrary.Conv_IntToText` (`self.Points to Add`)))
  (`KismetSystemLibrary.Delay` (`WidgetAnimation.GetEndTime` _points_animation))
  (`self.K2_DestroyActor`))

(fn `UserConstructionScript`)