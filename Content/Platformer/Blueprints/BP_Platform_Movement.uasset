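; Moving platform actor for a platformer, sliding a Platform component between a start and an end location.
; On BeginPlay it sets a timeline's play rate from a variable and starts it.
; Each timeline update uses the Movement track as the alpha to lerp between the two locations, setting the component's relative location without sweep.
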(event `self.ReceiveBeginPlay`
  (`TimelineComponent.SetPlayRate` (`self.Plantform Movement`) (`self.Play Rate`))
  (bind (_direction _movement) (`Timeline|Plantform Movement`)
    (:`Update`
      (`SceneComponent.K2_SetRelativeLocation` (`self.Platform`) (`KismetMathLibrary.VLerp` (`self.Loc_Start`) (`self.Loc_End`) _movement) false false))))

(fn `UserConstructionScript`
  (`parent.UserConstructionScript`))