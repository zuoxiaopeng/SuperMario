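; Mushroom platform that launches the player character when landed on and can be jumped through from below.
; A bottom overlap volume disables the cap's collision while the player is inside it.
; Top hits trigger a DoOnce-gated launch, dust emitter and timeline-driven cap scale animation, with a delayed reset re-arming the gate.
; The construction script scales the cap and stacks instanced trunk segments downward based on TrunkEndPoint's length.
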(event `self.CollisionBottom.OnComponentBeginOverlap`
  (params (OverlappedComponent :type "PrimitiveComponent Object Reference") (OtherActor :type "Actor Object Reference") (OtherComp :type "PrimitiveComponent Object Reference") (OtherBodyIndex :type Integer) (bFromSweep :type Boolean) (SweepResult :type "HitResult Structure (by ref)"))
  ; Jump UP Through The MushTop
  (if (== OtherActor (`GameplayStatics.GetPlayerCharacter` 0))
    (`PrimitiveComponent.SetCollisionEnabled` (`self.MushTop`) "NoCollision")))

(event `self.CollisionBottom.OnComponentEndOverlap`
  (params (OverlappedComponent :type "PrimitiveComponent Object Reference") (OtherActor :type "Actor Object Reference") (OtherComp :type "PrimitiveComponent Object Reference") (OtherBodyIndex :type Integer))
  ; Jump UP Through The MushTop
  (if (== (`GameplayStatics.GetPlayerCharacter` 0) OtherActor)
    (`PrimitiveComponent.SetCollisionEnabled` (`self.MushTop`) "QueryAndPhysics")))

(event `self.MushTop.OnComponentHit`
  (params (HitComponent :type "PrimitiveComponent Object Reference") (OtherActor :type "Actor Object Reference") (OtherComp :type "PrimitiveComponent Object Reference") (NormalImpulse :type "Vector Structure") (Hit :type "HitResult Structure (by ref)"))
  (bind _returnvalue (`GameplayStatics.GetPlayerCharacter` 0))
  (bind (_bblockinghit _binitialoverlap _time _distance _location _impactpoint _normal) (`GameplayStatics.BreakHitResult` Hit))
  ; MushTop Launcher
  (if (and (== OtherActor _returnvalue) (`KismetMathLibrary.EqualExactly_VectorVector` _normal (0.0 0.0 -1.0)))
    (`/Engine/EditorBlueprintResources/StandardMacros.DoOnce` false :!label _label
      (:`Completed`
        (`Character.LaunchCharacter` _returnvalue (`self.Launch_Valocity`) false false)
        (`GameplayStatics.SpawnEmitterAtLocation` "/Game/StarterContent/Particles/P_Ambient_Dust.P_Ambient_Dust" _location)
        (bind (_direction _mushtoptrace) (`Timeline|MushTopTimeline` :!via `PlayFromStart`)
          (:`Update`
            (`SceneComponent.SetRelativeScale3D` (`self.MushTop`) (`KismetMathLibrary.MakeVector` (* _mushtoptrace (`self.MushTop_Scale_X`)) (* _mushtoptrace (`self.MushTop_Scale_Y`)) (* _mushtoptrace (`self.MushTop_Scale_Z`))))
            (`KismetSystemLibrary.Delay` 0.2)
            (`self.ResetLauncher`)))))))

(event `ResetLauncher`
  ; MushTop Launcher
  (goto _label :!via `Reset`))

(fn `UserConstructionScript`
  ; Automatically Generate Tree Trunks
  (`SceneComponent.SetWorldScale3D` (`self.MushTop`) (`KismetMathLibrary.MakeVector` (`self.MushTop_Scale_X`) (`self.MushTop_Scale_Y`) (`self.MushTop_Scale_Z`)))
  (for _index (range (+ (`KismetMathLibrary.FTrunc` (/ (`KismetMathLibrary.VSize` (`self.TrunkEndPoint`)) 100.0)) 1))
    (`InstancedStaticMeshComponent.AddInstance` (`self.MushTrunk`) (`KismetMathLibrary.MakeTransform` (`KismetMathLibrary.MakeVector` 0.0 0.0 (* _index -100.0))) false)))