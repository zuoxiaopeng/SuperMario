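; BP_FireBar is a rotating platformer hazard that knocks back the third-person character and adjusts its hit points on contact.
; The construction script stacks instanced flame balls along local Z, stretches the hit box to cover them and applies the configurable rotation rate.
; Box overlap overwrites the character's movement velocity and calls AdjustHitPoints, with a DoOnce reset after a delay acting as the hit cooldown.
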(event `self.Box.OnComponentBeginOverlap`
  (params (OverlappedComponent :type "PrimitiveComponent Object Reference") (OtherActor :type "Actor Object Reference") (OtherComp :type "PrimitiveComponent Object Reference") (OtherBodyIndex :type Integer) (bFromSweep :type Boolean) (SweepResult :type "HitResult Structure (by ref)"))
  ; Hit by Fire Bar
  (bind _asbp_third_person_character (cast `/Game/ThirdPerson/Blueprints/BP_ThirdPersonCharacter` OtherActor))
  (`/Engine/EditorBlueprintResources/StandardMacros.DoOnce` false :!label _label
    (:`Completed`
      (set `MovementComponent.Velocity` (`self.Player Hit Velocity`) (`Character.CharacterMovement` _asbp_third_person_character))
      (`/Game/ThirdPerson/Blueprints/BP_ThirdPersonCharacter.Adjust Hit Points` _asbp_third_person_character (`self.Hit Points Adjustment to Player`))
      (`KismetSystemLibrary.Delay` (`self.Hit Cooldown`))
      (goto _label :!via `Reset`))))

(fn `UserConstructionScript`
  (bind _box (`self.Box`))
  (for _index (range (`self.Flame Ball Number`))
    (`|ExecutionSequence`
      (:`then_0`
        ; Add Instance of "Flame Ball"
        (`InstancedStaticMeshComponent.AddInstance` (`self.InstancedStaticMesh`) (`KismetMathLibrary.MakeTransform` (`KismetMathLibrary.MakeVector` 0.0 0.0 (`KismetMathLibrary.Conv_IntToDouble` (* _index (`self.Flame Ball Distance`)))) (struct) (`self.Flame Ball Size`)) false))
      (:`then_1`
        (bind _returnvalue (`KismetMathLibrary.Conv_IntToDouble` (/ (* (+ _index 1) (`self.Flame Ball Distance`)) 2)))
        ; Box Extent Sizing
        (`SceneComponent.K2_SetRelativeLocation` _box (`KismetMathLibrary.MakeVector` 0.0 0.0 _returnvalue) false false)
        (`BoxComponent.SetBoxExtent` _box (`KismetMathLibrary.MakeVector` 32.0 32.0 _returnvalue) true))
      (:`then_2`
        ; Allow Custom Rotation Rate
        (set `RotatingMovementComponent.RotationRate` (`self.Rotation Rate`) (`self.RotatingMovement`))))))